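; Player controller for a voice chat test that sets up positional VOIP with push-to-talk.
; P adds a VOIP talker, retries until PlayerState is valid, then registers it and attaches its voice to the player 0 character's capsule with attenuation and source effects.
; Holding V toggles speaking through console commands.
; O flip-flops OSS voice loopback for hearing one's own voice.
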(event `Key|P`
  (params (Key :type "Key Structure"))
  (bind _playerstate (`self.PlayerState`))
  (:`Pressed`
    (bind _returnvalue (`AddComponent|NODE_AddVOIPTalker-0`))
    (bind _output_get (set `self.VoipTalker_PlayerController` _returnvalue))
    (`/Engine/EditorBlueprintResources/StandardMacros.IsValid` _playerstate :!label _label
      (:`Is Valid`
        (`VOIPTalker.RegisterWithPlayerState` _output_get _playerstate)
        (`VOIPStatics.SetMicThreshold` -1.0)
        (bind _asbp_third_person_character_voice_chat (cast `/Game/_Project/Blueprints/VoiceChat_Test/BP_ThirdPersonCharacter_VoiceChat` (`GameplayStatics.GetPlayerCharacter` 0)))
        (set `VOIPTalker.Settings` (make `VoiceSettings` (`Character.CapsuleComponent` _asbp_third_person_character_voice_chat) "/Game/_Project/Blueprints/VoiceChat_Test/SA_VoiceChat.SA_VoiceChat" "/Game/_Project/Blueprints/VoiceChat_Test/SoundEffectSourcePresetChain.SoundEffectSourcePresetChain") (`self.VoipTalker_PlayerController`)))
      (:`Is Not Valid`
        (`KismetSystemLibrary.Delay` 0.2)
        (goto _label)))))

(event `self.ReceiveBeginPlay`)

(event `Key|V`
  (params (Key :type "Key Structure"))
  (:`Pressed`
    (`KismetSystemLibrary.ExecuteConsoleCommand` "ToggleSpeaking 1" null))
  (:`Released`
    (`KismetSystemLibrary.ExecuteConsoleCommand` "ToggleSpeaking 0" null)))

(event `Key|O`
  (params (Key :type "Key Structure"))
  (:`Pressed`
    (`/Engine/EditorBlueprintResources/StandardMacros.FlipFlop`
      (:`A`
        (`KismetSystemLibrary.ExecuteConsoleCommand` "OSS.VoiceLoopback 1 " null))
      (:`B`
        (`KismetSystemLibrary.ExecuteConsoleCommand` "OSS.VoiceLoopback 0" null)))))

(fn `UserConstructionScript`)