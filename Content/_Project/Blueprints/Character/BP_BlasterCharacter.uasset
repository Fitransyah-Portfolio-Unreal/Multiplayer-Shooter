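; BP_BlasterCharacter is the player character Blueprint, adding an overhead name display and proximity-style VOIP voice chat.
; On BeginPlay it polls until player 0's PlayerState is valid, then writes that player's name to the overhead widget.
; Debug-style keys drive voice: V is push-to-talk, O toggles loopback, and P creates a VOIPTalker registered to the PlayerState, attached to the capsule with attenuation and effects.
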(event `self.ReceiveBeginPlay`
  (bind _playerstate (`Controller.PlayerState` (`GameplayStatics.GetPlayerController` 0)))
  ;[1 1 1] Overhead widget call
  (bind _aswbp_overhead_widget (cast `/Game/_Project/Blueprints/HUD/WBP_OverheadWidget` (`WidgetComponent.GetUserWidgetObject` (`self.OverheadWidget`))))
  (`/Engine/EditorBlueprintResources/StandardMacros.IsValid` _playerstate :!label _label
    (:`Is Valid`
      (`OverheadWidget.SetDisplayText` _aswbp_overhead_widget (`PlayerState.GetPlayerName` _playerstate)))
    (:`Is Not Valid`
      (`KismetSystemLibrary.Delay` 0.2)
      (goto _label))))

(event `self.ReceiveTick`
  (params (DeltaSeconds :type "Float (single-precision)")))

(event `Key|V`
  (params (Key :type "Key Structure"))
  ;[1 1 1] Voice Chat
  (:`Pressed`
    (`KismetSystemLibrary.ExecuteConsoleCommand` "ToggleSpeaking 1" null))
  (:`Released`
    (`KismetSystemLibrary.ExecuteConsoleCommand` "ToggleSpeaking 0" null)))

(event `Key|O`
  (params (Key :type "Key Structure"))
  ;[1 1 1] Voice Chat
  (:`Pressed`
    (`/Engine/EditorBlueprintResources/StandardMacros.FlipFlop`
      (:`A`
        (`KismetSystemLibrary.ExecuteConsoleCommand` "OSS.VoiceLoopback 1 " null))
      (:`B`
        (`KismetSystemLibrary.ExecuteConsoleCommand` "OSS.VoiceLoopback 0" null)))))

(event `Key|P`
  (params (Key :type "Key Structure"))
  ;[1 1 1] Voice Chat
  (:`Pressed`
    (bind _returnvalue (`AddComponent|NODE_AddVOIPTalker-1`))
    (bind _output_get (set `self.VOIPTalker` _returnvalue))
    (`/Engine/EditorBlueprintResources/StandardMacros.IsValid` _output_get :!label _label_2
      (:`Is Valid`
        (`VOIPTalker.RegisterWithPlayerState` _output_get (`self.PlayerState`))
        (`VOIPStatics.SetMicThreshold` -1.0)
        (set `VOIPTalker.Settings` (make `VoiceSettings` (`self.CapsuleComponent`) "/Game/_Project/Blueprints/VoiceChat_Test/SA_VoiceChat.SA_VoiceChat" "/Game/_Project/Blueprints/VoiceChat_Test/SoundEffectSourcePresetChain.SoundEffectSourcePresetChain") (`self.VOIPTalker`)))
      (:`Is Not Valid`
        (`KismetSystemLibrary.Delay` 0.2)
        (goto _label_2)))))

(fn `UserConstructionScript`)